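; Base enemy Blueprint providing a ranged-checked, cooldown-gated montage attack and a death notification.
; TryAttack plays AttackMontage when the target is valid and within AttackRange, locking CanAttack and starting a cooldown timer.
; AttackSphere overlap with BP_MainCharacter subtracts Damage from Health, guarded by AlreadyHitThisSwing, which nothing here resets.
; Die fires the OnEnemyDied dispatcher and destroys the actor, but is not called within this Blueprint.
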(event OnComponentBeginOverlap(AttackSphere)
  (params (OverlappedComponent :type Primitive%20Component%20Object%20Reference) (OtherActor :type Actor%20Object%20Reference) (OtherComp :type Primitive%20Component%20Object%20Reference) (OtherBodyIndex :type Integer) (bFromSweep :type Boolean) (SweepResult :type Hit%20Result%20Structure%20%28by%20ref%29))
  (if (not (Variables|Default|GetbAlreadyHitThisSwing))
    (Utilities|Casting|CastToBP_MainCharacter OtherActor)
    (Variables|Default|SetbAlreadyHitThisSwing true)
    (Variables|Default|SetHealth (- (Variables|Default|GetHealth) (Variables|Default|GetDamage)))))

(event Custom|ResetCanAttack
  (Variables|Default|SetbCanAttack true))

(event EventBeginPlay)

(event Collision|EventActorBeginOverlap
  (params (OtherActor :type Actor%20Object%20Reference)))

(event EventTick
  (params (DeltaSeconds :type Float%20%28single-precision%29)))

(fn ConstructionScript)

(fn TryAttack
  (params (TargetActor :type Actor%20Object%20Reference))
  (if (Variables|Default|GetbCanAttack)
    (Utilities|IsValid TargetActor
      (:Is%20Valid
        (if (> (Math|Vector|VectorLength (- (Transformation|GetActorLocation) (Transformation|GetActorLocation TargetActor))) (Variables|Default|GetAttackRange))
          (return)
          (else
            (Variables|Default|SetbCanAttack false)
            (Animation|Montage|MontagePlay (Components|SkeletalMesh|GetAnimInstance (Variables|Character|GetMesh)) (Variables|Default|GetAttackMontage) 1.0 "MontageLength" 0.0 true)
            (Utilities|Time|SetTimerbyEvent (EventDispatchers|CreateEvent :!event Custom|ResetCanAttack) (Variables|Default|GetAttackCooldown)))))
      (:Is%20Not%20Valid
        (return)))
    (else
      (return))))

(fn Die
  (Default|CallOnEnemyDied)
  (Actor|DestroyActor))