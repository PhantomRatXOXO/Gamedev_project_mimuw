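; Main character Blueprint that leaves a fire trail when dashing and points a guide arrow at the exit gate.
; OnDashStart runs a short looping timer that spawns BP_FireHazard at the character's transform, then clears it after a brief delay.
; BeginPlay sets the first BP_ExitGate found as the GuideArrow child actor's target, then starts a camera fade-in.
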(event Custom|SpawnFireEvent
  (Game|SpawnActorfromClass "/Game/DashVisuals/BP_FireHazard.BP_FireHazard_C" (Transformation|GetActorTransform) "Undefined" "MultiplyWithRoot" 0 0))

(event EventBeginPlay
  (bind _outactors (Actor|GetAllActorsOfClass "/Game/Levels/Level3/BP_ExitGate.BP_ExitGate_C"))
  (bind _asbp_guide_arrow (Utilities|Casting|CastToBP_GuideArrow (Variables|/Script/Engine.ChildActorComponent|GetChildActor (Variables|Default|GetGuideArrow))))
  (Variables|/Game/Characters/MainCharacter/BP_GuideArrow.BP_GuideArrow_C|SetTargetGate _asbp_guide_arrow (Utilities|Array|Get(acopy) _outactors))
  (CameraFades|StartCameraFade :self (Game|GetPlayerCameraManager 0) :FromAlpha 2.0 :Duration 2.0))

(event Collision|EventActorBeginOverlap
  (params (OtherActor :type Actor%20Object%20Reference)))

(event EventTick
  (params (DeltaSeconds :type Float%20%28single-precision%29)))

(event EventOnDashStart
  (bind _returnvalue (Utilities|Time|SetTimerbyEvent (delegate Custom|SpawnFireEvent) 0.05 true))
  (bind _output_get (Variables|Default|SetFireTimerHandle _returnvalue))
  (Utilities|FlowControl|Delay 0.5)
  (Utilities|Time|ClearandInvalidateTimerbyHandle _output_get))

(fn ConstructionScript)